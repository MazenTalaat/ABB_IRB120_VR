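; ROS-style string topic subscriber that receives six joint values, apparently for a robot with VR goal control.
; On construct it initializes on /joints and subscribes, then calls Init again for /vr_goal with no further Subscribe.
; Each string message is split on commas through nested Split calls into Joint1 to Joint6 floats.
; It then records the receive time and raises the NewTime flag.
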(event `self.OnConstruct`
  (`self.Init` "/joints" "String" 144)
  (`self.Subscribe`)
  (`self.Init` "/vr_goal" "String" 144))

(event `self.OnStringMessage`
  (params (Data :type String))
  (bind (_lefts _rights) (`KismetStringLibrary.Split` Data ","))
  (bind (_lefts_2 _rights_2) (`KismetStringLibrary.Split` _rights ","))
  (bind (_lefts_3 _rights_3) (`KismetStringLibrary.Split` _rights_2 ","))
  (bind (_lefts_4 _rights_4) (`KismetStringLibrary.Split` _rights_3 ","))
  (bind (_lefts_5 _rights_5) (`KismetStringLibrary.Split` _rights_4 ","))
  (set `self.Joint1` (`KismetStringLibrary.Conv_StringToDouble` _lefts))
  (set `self.Joint2` (`KismetStringLibrary.Conv_StringToDouble` _lefts_2))
  (set `self.Joint3` (`KismetStringLibrary.Conv_StringToDouble` _lefts_3))
  (set `self.Joint4` (`KismetStringLibrary.Conv_StringToDouble` _lefts_4))
  (set `self.Joint5` (`KismetStringLibrary.Conv_StringToDouble` _lefts_5))
  (set `self.Joint6` (`KismetStringLibrary.Conv_StringToDouble` _rights_5))
  (set `self.ReceivedTime` (`KismetMathLibrary.Now`))
  (set `self.NewTime` true))