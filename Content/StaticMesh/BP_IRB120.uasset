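; Six-axis IRB120 robot arm actor whose pose mirrors joint values from a BP_Sub data object, apparently fed by ROS.
; BeginPlay constructs the BP_Sub with the player pawn as outer and stores it as ROSData.
; Each Tick converts the joint radians to degrees, negating Joint1, and sets each part's relative rotation about its single axis.
; Per-joint limit clamping and debug printing exist but are disconnected.
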(event `self.ReceiveBeginPlay`
  (bind _returnvalue (`|GenericCreateObject` "/Game/BP_Sub.BP_Sub_C" (`GameplayStatics.GetPlayerPawn` 0)))
  (set `self.ROS_Data` _returnvalue))

(event `self.ReceiveTick`
  (params (DeltaSeconds :type "Float (single-precision)"))
  (bind _ros_data (`self.ROS_Data`))
  (set `self.P1_ZAngle` (`KismetMathLibrary.RadiansToDegrees` (* -1.0 (`/Game/BP_Sub.Joint1` _ros_data))))
  (set `self.P2_XAngle` (`KismetMathLibrary.RadiansToDegrees` (* 1.0 (`/Game/BP_Sub.Joint2` _ros_data))))
  (set `self.P3_XAngle` (`KismetMathLibrary.RadiansToDegrees` (* 1.0 (`/Game/BP_Sub.Joint3` _ros_data))))
  (set `self.P4_YAngle` (`KismetMathLibrary.RadiansToDegrees` (* 1.0 (`/Game/BP_Sub.Joint4` _ros_data))))
  (set `self.P5_XAngle` (`KismetMathLibrary.RadiansToDegrees` (* 1.0 (`/Game/BP_Sub.Joint5` _ros_data))))
  (set `self.P6_YAngle` (`KismetMathLibrary.RadiansToDegrees` (* 1.0 (`/Game/BP_Sub.Joint6` _ros_data))))
  (`self.P1_Control`)
  (`self.P2_Control`)
  (`self.P3_Control`)
  (`self.P4_Control`)
  (`self.P5_Control`)
  (`self.P6_Control`))

(fn `P1_Control`
  (`SceneComponent.K2_SetRelativeRotation` (`self.P1`) (`KismetMathLibrary.MakeRotator` 0.0 0.0 (`self.P1_ZAngle`)) false false))

(fn `P2_Control`
  (`SceneComponent.K2_SetRelativeRotation` (`self.P2`) (`KismetMathLibrary.MakeRotator` (`self.P2_XAngle`)) false false))

(fn `P3_Control`
  (`SceneComponent.K2_SetRelativeRotation` (`self.P3`) (`KismetMathLibrary.MakeRotator` (`self.P3_XAngle`)) false false))

(fn `P4_Control`
  (`SceneComponent.K2_SetRelativeRotation` (`self.P4`) (`KismetMathLibrary.MakeRotator` 0.0 (`self.P4_YAngle`)) false false))

(fn `P5_Control`
  (`SceneComponent.K2_SetRelativeRotation` (`self.P5`) (`KismetMathLibrary.MakeRotator` (`self.P5_XAngle`)) false false))

(fn `P6_Control`
  (`SceneComponent.K2_SetRelativeRotation` (`self.P6`) (`KismetMathLibrary.MakeRotator` 0.0 (`self.P6_YAngle`)) false false))

(fn `UserConstructionScript`)